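; Component that keeps a running point total, named as a fragments counter, for the actor that owns it.
; AgregarPuntos adds to Puntos and prints the amount added with the new total, RestarPuntos subtracts without any clamp, and GetPuntos returns the current value.
; The event graph is empty, so the total changes only when these functions are called.
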(event EventBeginPlay)

(event EventTick
  (params (DeltaSeconds :type Float%20%28single-precision%29)))

(fn AgregarPuntos
  (params (puntos%20a%20sumar :type Integer))
  (bind _output_get (Variables|Default|SetPuntos (+ (Variables|Default|GetPuntos) puntos%20a%20sumar)))
  (Development|PrintString (Utilities|String|Append "Se sumaron puntos" (Utilities|String|ToString(Integer) puntos%20a%20sumar) " 
Los puntos totales son: 
" (Utilities|String|ToString(Integer) _output_get))))

(fn RestarPuntos
  (params (Puntos%20a%20restar :type Integer))
  (Variables|Default|SetPuntos (- (Variables|Default|GetPuntos) Puntos%20a%20restar)))

(fn GetPuntos
  (return (Variables|Default|GetPuntos)))